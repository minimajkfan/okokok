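; Spikes hazard Blueprint that kills the player by restarting the current level when its cone is hit.
; The first hit on the cone, with no check on what hit it, fades the camera to red, waits briefly, then reopens the level by name.
; On BeginPlay, the Miganie timeline makes the point light flicker by lerping its intensity between the Migotanie value and zero.
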(event `self.Cone.OnComponentHit`
  (params (HitComponent :type "PrimitiveComponent Object Reference") (OtherActor :type "Actor Object Reference") (OtherComp :type "PrimitiveComponent Object Reference") (NormalImpulse :type "Vector Structure") (Hit :type "HitResult Structure (by ref)"))
  ;[0.3615 0.6995 1] Dying
  (`/Engine/EditorBlueprintResources/StandardMacros.DoOnce` false
    (:`Completed`
      (bind _returnvalue (`GameplayStatics.GetCurrentLevelName` true))
      (`PlayerCameraManager.StartCameraFade` (`PlayerController.PlayerCameraManager` (`GameplayStatics.GetPlayerController` 0)) 0.0 1.0 1.0 (struct :`R` 1.0 :`A` 1.0) false true)
      (`KismetSystemLibrary.Delay` 1.0)
      (`GameplayStatics.OpenLevel` (`KismetStringLibrary.Conv_StringToName` _returnvalue)))))

(event `self.ReceiveBeginPlay`
  (bind (_direction _migmig) (`Timeline|Miganie` :!via `PlayFromStart`)
    (:`Update`
      (`LightComponent.SetIntensity` (`self.PointLight`) (`KismetMathLibrary.Lerp` (`self.Migotanie`) 0.0 _migmig)))))

(fn `UserConstructionScript`)