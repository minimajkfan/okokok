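; Fall-death trigger actor that restarts the current level when an overlap with its FallTrigger component ends.
; On end overlap, with no filter on the overlapping actor, it starts a camera fade to red and reopens the level by name after a delay shorter than the fade.
; On BeginPlay it fades the camera in from near-white, which also covers the restart.
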(event `self.fallTrigger.OnComponentEndOverlap`
  (params (OverlappedComponent :type "PrimitiveComponent Object Reference") (OtherActor :type "Actor Object Reference") (OtherComp :type "PrimitiveComponent Object Reference") (OtherBodyIndex :type Integer))
  ;[1 0.2708 0.392] Dying
  (bind _returnvalue (`GameplayStatics.GetCurrentLevelName` true))
  (`PlayerCameraManager.StartCameraFade` (`PlayerController.PlayerCameraManager` (`GameplayStatics.GetPlayerController` 0)) 0.0 1.0 2.0 (struct :`R` 1.0 :`A` 1.0) false false)
  (`KismetSystemLibrary.Delay` 1.0)
  (`GameplayStatics.OpenLevel` (`KismetStringLibrary.Conv_StringToName` _returnvalue)))

(event `self.ReceiveBeginPlay`
  ;[1 0.7149 0.3122] Stay determined
  (`PlayerCameraManager.StartCameraFade` (`PlayerController.PlayerCameraManager` (`GameplayStatics.GetPlayerController` 0)) 1.0 0.0 2.0 (struct :`R` 0.96706 :`G` 1.0 :`B` 0.989879 :`A` 1.0) false false))

(fn `UserConstructionScript`)